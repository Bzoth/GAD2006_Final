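; Boss character Blueprint that links damage, hit reactions, death and a phase change to its AI Blackboard and behavior tree.
; BeginPlay stores the player in the Blackboard; Tick prints health and flags OutOfRange when the range check fails.
; Damage feeds TakeDamage, TookHeavyDamage and ExplodeTransition, while hit reactions gate further hits and can halt movement during a montage.
; Death stops AI logic; phase change clears Phase1, plays a swap montage, then reruns BT_Boss.
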(event EventTick
  (params (DeltaSeconds :type Float%20%28single-precision%29))
  (Development|PrintString (Utilities|String|ToString(Float) (Variables|Default|GetCurrentHealth)) true true "(R=0.000000,G=0.660000,B=1.000000,A=1.000000)" 2.0 "a")
  (bind _returnvalue (Class|EnemyBoss|CheckinRange (Game|GetPlayerCharacter 0)))
  (if (not _returnvalue)
    (AI|Components|Blackboard|SetValueasBool (AI|GetBlackboard 0) (Utilities|Name|MakeLiteralName "OutOfRange") true)))

(event EventBeginPlay
  (AI|Components|Blackboard|SetValueasObject (AI|GetBlackboard 0) (Utilities|Name|MakeLiteralName "Player") (Game|GetPlayerCharacter 0)))

(event EventDamagetoEnemy
  (params (DamageAmount :type Float%20%28double-precision%29) (HitLocation :type Vector :default "0, 0, 0"))
  (bind _returnvalue (Class|EnemyBase|TakeDamage DamageAmount))
  (Class|EnemyBoss|TookHeavyDamage _returnvalue)
  (Class|EnemyBoss|ExplodeTransition))

(event EventOnHitReact
  (Variables|Default|SetCanTakeHit false)
  (if (Variables|Default|GetCanHitAnim)
    (Variables|Default|SetCanHitAnim false)
    (Animation|Montage|PlayMontage (Variables|Character|GetMesh) "/Game/Assets/Boss/AM_BossTakeHit.AM_BossTakeHit"
      (:then
        (Variables|/Script/Engine.CharacterMovementComponent|SetMaxWalkSpeed (Variables|Character|GetCharacterMovement) 0.0))
      (:OnCompleted
        (Variables|Default|SetCanTakeHit true :!label _label)
        (Variables|/Script/Engine.CharacterMovementComponent|SetMaxWalkSpeed (Variables|Character|GetCharacterMovement) 4e+02))
      (:OnInterrupted
        (goto _label)))
    (else
      (Utilities|FlowControl|Delay 0.2)
      (Variables|Default|SetCanTakeHit true))))

(event EventOnDeath
  (bind _self self)
  (bind _returnvalue (AI|GetAIController _self))
  (Animation|StopAnimMontage (Animation|GetCurrentMontage :!class /Script/Engine.Character))
  (Animation|Montage|PlayMontage (Variables|Character|GetMesh) "/Game/Assets/Boss/AM_BossDeath.AM_BossDeath"
    (:then
      (AI|Logic|StopLogic (Variables|/Script/AIModule.AIController|GetBrainComponent _returnvalue) "")
      (AI|ClearFocus _returnvalue))))

(event EventPhaseChanged
  (bind _returnvalue (Animation|GetCurrentMontage :!class /Script/Engine.Character))
  (Variables|Default|SetCanTakeHit false)
  (Utilities|FlowControl|Delay 1.0)
  (AI|Components|Blackboard|SetValueasBool (AI|GetBlackboard 0) (Utilities|Name|MakeLiteralName "Phase1") false)
  (AI|Logic|StopLogic (Variables|/Script/AIModule.AIController|GetBrainComponent (AI|GetAIController self)) "")
  (Utilities|IsValid _returnvalue
    (:Is%20Valid
      (Animation|StopAnimMontage _returnvalue))
    (:Is%20Not%20Valid
      _))
  (Animation|Montage|PlayMontage (Variables|Character|GetMesh) "/Game/Assets/Boss/AM_PhaseSwap.AM_PhaseSwap"
    (:OnCompleted
      _)
    (:OnInterrupted
      _))
  (Utilities|FlowControl|Delay 1.0)
  (Variables|Default|SetCanTakeHit true)
  (AI|RunBehaviorTree (AI|GetAIController self) "/Game/Blueprints/Boss/BT_Boss.BT_Boss"))

(fn ConstructionScript)