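; BP_BossActivator is a one-shot trigger actor that starts the boss fight when the player overlaps it.
; It finds the boss, runs its behavior tree, stores the player in the blackboard and sets the AI controller's focus on the player.
; It then reveals the boss health bar in the player's UI and destroys itself.
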(event Collision|EventActorBeginOverlap
  (params (OtherActor :type Actor%20Object%20Reference))
  (if (== OtherActor (Game|GetPlayerCharacter 0))
    (bind _returnvalue (Actor|GetActorOfClass "/Game/Blueprints/Boss/BP_Boss.BP_Boss_C"))
    (AI|RunBehaviorTree (AI|GetAIController _returnvalue) "/Game/Blueprints/Boss/BT_Boss.BT_Boss")
    (AI|Components|Blackboard|SetValueasObject (AI|GetBlackboard _returnvalue) (Utilities|Name|MakeLiteralName "Player") (Game|GetPlayerCharacter 0))
    (AI|SetFocus (AI|GetAIController _returnvalue) (Game|GetPlayerCharacter 0))
    (bind _returnvalue_2 (Actor|GetActorOfClass "/Game/Blueprints/Player/BP_PlayerCharacter.BP_PlayerCharacter_C"))
    (Widget|SetVisibility (Variables|/Game/Blueprints/Player/WBP_PlayerUI.WBP_PlayerUI_C|GetBossHP (Variables|/Game/Blueprints/Player/BP_PlayerCharacter.BP_PlayerCharacter_C|GetPlayerUI _returnvalue_2)) "Visible")
    (Actor|DestroyActor)))

(fn ConstructionScript)