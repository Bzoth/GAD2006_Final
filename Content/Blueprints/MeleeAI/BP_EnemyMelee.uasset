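; Melee enemy Blueprint that links damage, hit reactions, death and player detection to its AI Blackboard.
; BeginPlay writes two patrol points to the Blackboard, and pawn sensing sets the Player key on sighting the player.
; DamagetoEnemy forwards to TakeDamage, while OnHitReact plays a montage, re-enables CanTakeHit after a short delay and, once only, also sets the Player key.
; OnDeath plays the death montage.
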(event OnSeePawn(PawnSensing)
  (params (Pawn :type Pawn%20Object%20Reference))
  (if (== Pawn (Game|GetPlayerCharacter 0))
    (AI|Components|Blackboard|SetValueasObject (AI|GetBlackboard 0) (Utilities|Name|MakeLiteralName "Player") (Game|GetPlayerCharacter 0))))

(event EventBeginPlay
  (bind _returnvalue (AI|GetBlackboard 0))
  (AI|Components|Blackboard|SetValueasObject _returnvalue (Utilities|Name|MakeLiteralName "Patrol1") (Variables|Default|GetPatrol1))
  (AI|Components|Blackboard|SetValueasObject _returnvalue (Utilities|Name|MakeLiteralName "Patrol2") (Variables|Default|GetPatrol2)))

(event EventDamagetoEnemy
  (params (DamageAmount :type Float%20%28double-precision%29) (HitLocation :type Vector :default "0, 0, 0"))
  (Class|EnemyBase|TakeDamage DamageAmount))

(event EventOnHitReact
  (Animation|Montage|PlayMontage (Variables|Character|GetMesh) "/Game/Assets/EnemyMelee/AM_MeleeEnemyReaction_Hit.AM_MeleeEnemyReaction_Hit"
    (:then
      (Utilities|FlowControl|Delay 0.3)
      (Variables|Default|SetCanTakeHit true)
      (Utilities|FlowControl|DoOnce false
        (:Completed
          (AI|Components|Blackboard|SetValueasObject (AI|GetBlackboard 0) (Utilities|Name|MakeLiteralName "Player") (Game|GetPlayerCharacter 0)))))))

(event EventOnDeath
  (Animation|Montage|PlayMontage (Variables|Character|GetMesh) "/Game/Assets/EnemyMelee/AM_MeleeEnemyDeath.AM_MeleeEnemyDeath"))

(fn ConstructionScript)