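; Player character Blueprint that handles combat reactions, pickups and UI for the hero.
; BeginPlay creates the HUD and applies hat, color and stats from BP_GameInstance.
; Triggered events play attack, potion, hit and death montages, resetting action flags on completion, interruption or delay; dodge launches along current velocity.
; Montage notifies time traced special-magic damage and potion healing, which also fires on interruption; death disables input and shows a death screen.
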(event EventOnLightAttackTriggered
  (Animation|Montage|PlayMontage (Variables|Character|GetMesh) "/Game/Assets/Player/Montages/AM_Light1.AM_Light1"
    (:OnCompleted
      _)
    (:OnInterrupted
      _))
  (Variables|Default|SetCanAttack true))

(event EventOnDodgeTriggered
  (Character|LaunchCharacter (* (Transformation|GetVelocity) 1e+01) true false)
  (Utilities|FlowControl|Delay 3.0)
  (Variables|Default|SetCanDodge true))

(event EventCollectPotion
  (Class|CharacterBase|HealPotionPickup))

(event EventCollectMana
  (Class|CharacterBase|ManaPickup))

(event EventDamagetoPlayer
  (params (Damage :type Float%20%28double-precision%29))
  (Class|CharacterBase|TakeDamage Damage))

(event EventOnHeavyAttackTriggered
  (Animation|Montage|PlayMontage (Variables|Character|GetMesh) "/Game/Assets/Player/Montages/AM_Heavy.AM_Heavy" 0.8
    (:OnCompleted
      _)
    (:OnInterrupted
      _))
  (Variables|Default|SetCanAttack true))

(event EventBeginPlay
  (bind _returnvalue (UserInterface|CreateWidget "/Game/Blueprints/Player/WBP_PlayerUI.WBP_PlayerUI_C" 0 self))
  (bind _output_get (Variables|Default|SetPlayerUI _returnvalue))
  (UserInterface|Viewport|AddtoViewport _returnvalue 0)
  (bind _asbp_game_instance (Utilities|Casting|CastToBP_GameInstance (Game|GetGameInstance)))
  (Components|StaticMesh|SetStaticMesh (Variables|Default|GetHatMesh) (Variables|/Game/Blueprints/BP_GameInstance.BP_GameInstance_C|GetHat _asbp_game_instance))
  (bind _returnvalue_2 (Rendering|Material|CreateDynamicMaterialInstance (Variables|Character|GetMesh) 0 0 "None" :!class /Script/Engine.PrimitiveComponent))
  (Rendering|Material|SetVectorParameterValue _returnvalue_2 "Color" (Utilities|Struct|MakeLinearColor (.x (Variables|/Game/Blueprints/BP_GameInstance.BP_GameInstance_C|GetColor _asbp_game_instance)) (.y (Variables|/Game/Blueprints/BP_GameInstance.BP_GameInstance_C|GetColor _asbp_game_instance)) (.z (Variables|/Game/Blueprints/BP_GameInstance.BP_GameInstance_C|GetColor _asbp_game_instance)) 1.0) :!class /Script/Engine.MaterialInstanceDynamic)
  (Class|CharacterBase|SetStats (Variables|/Game/Blueprints/BP_GameInstance.BP_GameInstance_C|GetVigor _asbp_game_instance) (Variables|/Game/Blueprints/BP_GameInstance.BP_GameInstance_C|GetEndurance _asbp_game_instance) (Variables|/Game/Blueprints/BP_GameInstance.BP_GameInstance_C|GetStrenght _asbp_game_instance) (Variables|/Game/Blueprints/BP_GameInstance.BP_GameInstance_C|GetIntelligance _asbp_game_instance)))

(event EventOnSpecialAttackTriggered
  (Animation|Montage|PlayMontage (Variables|Character|GetMesh) "/Game/Assets/Player/Montages/AM_SpecialCombo.AM_SpecialCombo" 0.75
    (:OnCompleted
      _)
    (:OnInterrupted
      _))
  (Variables|Default|SetCanAttack true))

(event EventOnSpecialMagicTriggered
  (Animation|Montage|PlayMontage (Variables|Character|GetMesh) "/Game/Assets/Player/Montages/AM_HeavyCast.AM_HeavyCast"
    (:OnNotifyBegin
      (bind _returnvalue (Class|CharacterBase|SpecialMagicAttackTrace))
      (for _array_element _returnvalue
        (Class|BPIDamage|DamagetoEnemy(Message) (.Actor (Utilities|Struct|BreakAttackReturn _array_element)) (Variables|Default|GetDamage) (.HitLocation (Utilities|Struct|BreakAttackReturn _array_element)))))))

(event EventOnTakeHit
  (Utilities|IsValid (Animation|GetCurrentMontage :!class /Script/Engine.Character)
    (:Is%20Valid
      _)
    (:Is%20Not%20Valid
      (Animation|Montage|PlayMontage (Variables|Character|GetMesh) "/Game/Assets/Player/Montages/AM_TakeDamage.AM_TakeDamage" 1.0 0.0 "None" false
        (:then
          _))))
  (Utilities|FlowControl|Delay 0.6)
  (Variables|Default|SetCanTakeDamage true))

(event EventOnDeath
  (Collision|SetCollisionEnabled (Variables|Default|GetCapsuleComponent) "NoCollision")
  (Input|DisableInput (Game|GetPlayerController 0))
  (Animation|Montage|PlayMontage (Variables|Character|GetMesh) "/Game/Assets/Player/Montages/AM_Death.AM_Death" 1.0 0.0 "None" false
    (:then
      (Utilities|FlowControl|Delay 3.0)
      (bind _returnvalue (UserInterface|CreateWidget "/Game/Blueprints/Player/WBP_Death.WBP_Death_C"))
      (UserInterface|Viewport|AddtoViewport _returnvalue 0))))

(event EventOnPotionUsed
  (Animation|Montage|PlayMontage (Variables|Character|GetMesh) "/Game/Assets/Player/Montages/AM_DrinkPot.AM_DrinkPot" 1.0 0.0 "None" false
    (:OnCompleted
      (Variables|Default|SetCanAttack true :!label _label))
    (:OnInterrupted
      (Utilities|FlowControl|Sequence
        (:then_0
          (goto _label))
        (:then_1
          (Class|CharacterBase|Heal (Variables|Default|GetPotionHealAmount) :!label _label_2))))
    (:OnNotifyBegin
      (goto _label_2)))
  (Variables|Default|SetCanTakeDamage true))

(fn ConstructionScript)