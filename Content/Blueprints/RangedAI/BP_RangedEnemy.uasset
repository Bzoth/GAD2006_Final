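; BP_RangedEnemy is a ranged AI enemy that patrols, detects the player, reacts to hits and plays a death montage.
; It feeds two patrol points to its Blackboard on BeginPlay, then sets the Player key on PawnSensing sight or first hit reaction.
; Hit reactions re-enable CanTakeHit after a short delay.
; A looping timer, started on demand, polls line of sight, sets CanSeePlayer once true, then clears itself.
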(event OnSeePawn(PawnSensing)
  (params (Pawn :type Pawn%20Object%20Reference))
  (if (== Pawn (Game|GetPlayerCharacter 0))
    (AI|Components|Blackboard|SetValueasObject (AI|GetBlackboard 0) (Utilities|Name|MakeLiteralName "Player") (Game|GetPlayerCharacter 0))))

(event Custom|CanSeePlayerTimer
  (bind _returnvalue (Class|EnemyRanged|CanSeePlayer (Game|GetPlayerCharacter 0)))
  (if _returnvalue
    (AI|Components|Blackboard|SetValueasBool (AI|GetBlackboard 0) (Utilities|Name|MakeLiteralName "CanSeePlayer") true)
    (Utilities|Time|ClearandInvalidateTimerbyHandle (stale Custom|StartCheckingVision _returnvalue))))

(event Custom|StartCheckingVision
  (bind _returnvalue (Utilities|Time|SetTimerbyEvent (delegate Custom|CanSeePlayerTimer) 0.1 true)))

(event EventBeginPlay
  (bind _returnvalue (AI|GetBlackboard 0))
  (AI|Components|Blackboard|SetValueasObject _returnvalue (Utilities|Name|MakeLiteralName "Patrol1") (Variables|Default|GetPatrol1))
  (AI|Components|Blackboard|SetValueasObject _returnvalue (Utilities|Name|MakeLiteralName "Patrol2") (Variables|Default|GetPatrol2)))

(event EventOnHitReact
  (Animation|Montage|PlayMontage (Variables|Character|GetMesh) "/Game/Assets/EnemyRanged/AM_RangedHit.AM_RangedHit"
    (:then
      (Utilities|FlowControl|Delay 0.3)
      (Variables|Default|SetCanTakeHit true)
      (Utilities|FlowControl|DoOnce false
        (:Completed
          (AI|Components|Blackboard|SetValueasObject (AI|GetBlackboard 0) (Utilities|Name|MakeLiteralName "Player") (Game|GetPlayerCharacter 0)))))))

(event EventOnDeath
  (Animation|Montage|PlayMontage (Variables|Character|GetMesh) "/Game/Assets/EnemyRanged/AM_Death.AM_Death"))

(event EventDamagetoEnemy
  (params (DamageAmount :type Float%20%28double-precision%29) (HitLocation :type Vector :default "0, 0, 0"))
  (Class|EnemyBase|TakeDamage DamageAmount))

(fn ConstructionScript)